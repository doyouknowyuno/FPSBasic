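; Base weapon Blueprint that handles single and automatic fire, ammo and reloading.
; Firing runs a camera sphere trace, then a muzzle trace toward that aim point; automatic mode repeats it through a gated delay loop.
; Each shot spends ammo, then applies damage and effects, or stops the weapon on an empty clip.
; Authority refills the clip from reserve and spawns separate owner-visible and owner-hidden muzzle effects for first- and third-person meshes.
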(event Custom|OffWeaponFire
  (Utilities|FlowControl|Sequence
    (:then_0
      (Utilities|AutoFireMode) ; enters at Close
    )
    (:then_1
      (CallFunction|StopFX))))

(event Custom|OnWeaponFire
  (Development|PrintString "Fire")
  (switch Utilities|FlowControl|Switch|SwitchonE_FiringMode (Variables|Default|GetFiringMode)
    (:NewEnumerator0
      _)
    (:NewEnumerator1
      (Utilities|AutoFireMode
        (:Exit
          _))))
  (bind (_hit _outhit _fpmuzzlelocation _tpmuzzlelocation) (CallFunction|SphereTrace))
  (CallFunction|ShootInfo _hit _outhit _fpmuzzlelocation _tpmuzzlelocation))

(event Custom|ShootInfo
  (params (Hit :type Boolean) (OutHit :type Hit%20Result%20Structure) (FPMuzzle :type Vector) (TPMuzzle :type Vector))
  (Variables|Default|SetCurrentAmmoInClip (Math|Integer|Clamp(Integer) (- (Variables|Default|GetCurrentAmmoInClip) 1) 0 (Variables|Default|GetMaxAmmoClipSize)))
  (if (not (== (Variables|Default|GetCurrentAmmoInClip) 0))
    (Game|Damage|ApplyDamage (.HitActor (Collision|BreakHitResult OutHit)) 1e+01 (Game|GetInstigatorController) self)
    (CallFunction|StartFX Hit OutHit)
    (else
      (Default|StopWeapon (Variables|Default|GetBPMainCharacter)))))

(event Custom|StopFX
  (bind _tp_fx (Variables|Default|GetTP_FX))
  (bind _fp_fx (Variables|Default|GetFP_FX))
  (Utilities|FlowControl|Sequence
    (:then_0
      (Utilities|IsValid _fp_fx
        (:Is%20Valid
          (Actor|DestroyActor _fp_fx))))
    (:then_1
      (Utilities|IsValid _tp_fx
        (:Is%20Valid
          (Actor|DestroyActor _tp_fx))))))

(event Custom|StartFX
  (params (Hit :type Boolean) (HitResult :type Hit%20Result%20Structure))
  (CallFunction|FireFX Hit HitResult)
  (switch Utilities|FlowControl|Switch|SwitchonE_FiringMode (Variables|Default|GetFiringMode)
    (:NewEnumerator0
      (Utilities|FlowControl|Sequence
        (:then_0
          (Utilities|FlowControl|Delay (Variables|Default|GetFireRate))
          (CallFunction|StopFX))
        (:then_1
          (Audio|SpawnSound2D "/Game/MP_FPSBasic/Audio/Cues/A_S_Rifle_ShotEnd_Cue.A_S_Rifle_ShotEnd_Cue" 1.0 1.0 0.0 0))))))

(event Custom|OnReloadWeapon
  (CallFunction|ReloadFx)
  (Utilities|FlowControl|Delay 0.2)
  (CallFunction|ReloadAddAmmo))

(event Custom|ReloadFX
  (Audio|SpawnSound2D "/Game/MP_FPSBasic/Audio/Cues/A_Rifle_Reload_Cue.A_Rifle_Reload_Cue" 1.0 1.0 0.0 0))

(event EventBeginPlay
  (Variables|Default|SetCurrentMaxAmmo (Variables|Default|GetMaxAmmo))
  (Variables|Default|SetCurrentAmmoInClip (Variables|Default|GetMaxAmmoClipSize)))

(fn ConstructionScript)

(fn SphereTrace
  (bind _returnvalue (Game|GetPlayerCameraManager 0))
  (bind _returnvalue_2 (Components|GetOwner))
  (bind _returnvalue_3 (Math|Float|MakeLiteralFloat 2.0))
  (bind _sk_fp_mesh (Variables|Default|GetSK_FP_Mesh))
  (bind _returnvalue_4 (Camera|GetCameraLocation _returnvalue))
  (bind _returnvalue_5 (Transformation|GetSocketLocation _sk_fp_mesh "Muzzle"))
  (bind _array (Utilities|Array|MakeArray _returnvalue_2))
  (bind (_outhit _returnvalue_6) (Collision|SphereTraceByChannel _returnvalue_4 (+ (+ _returnvalue_4 (* (Math|Vector|GetForwardVector (Camera|GetCameraRotation _returnvalue)) 5e+03)) (* (Math|Random|RandomFloat) (Math|Random|RandomUnitVector))) _returnvalue_3 "TraceTypeQuery1" false _array "None"))
  (bind (_outhit_2 _returnvalue_7) (Collision|SphereTraceByChannel _returnvalue_5 (select _returnvalue_6 (.ImpactPoint (Collision|BreakHitResult _outhit)) (.TraceEnd (Collision|BreakHitResult _outhit))) _returnvalue_3 "TraceTypeQuery1" false _array "ForDuration"))
  (return _returnvalue_7 _outhit_2 _returnvalue_5 (Transformation|GetSocketLocation (Variables|Default|GetSk_TP_Mesh) "Muzzle")))

(fn FireFX
  (params (Hit :type Boolean) (HitResult :type Hit%20Result%20Structure))
  (bind (_bblockinghit _binitialoverlap _time _distance _location _impactpoint _normal _impactnormal) (Collision|BreakHitResult HitResult))
  (Utilities|FlowControl|Sequence
    (:then_0
      (Networking|SwitchHasAuthority
        (:Authority
          (Utilities|FlowControl|Sequence
            (:then_0
              (Utilities|IsValid (Variables|Default|GetFP_FX)
                (:Is%20Not%20Valid
                  (bind _returnvalue (Game|SpawnActorfromClass "/Game/Blueprints/Weapons/BP_FX_Fire.BP_FX_Fire_C" (Math|Transform|MakeTransform "0, 0, 0") "Undefined" (Components|GetOwner) 0))
                  (Transformation|AttachComponentToComponent _returnvalue (Variables|Default|GetSK_FP_Mesh) (Utilities|Name|MakeLiteralName "Muzzle") "SnapToTarget" "SnapToTarget" "SnapToTarget" true)
                  (bind _output_get (Variables|Default|SetFP_FX _returnvalue))
                  (Default|SetOwnerSee _output_get))))
            (:then_1
              (Utilities|IsValid (Variables|Default|GetTP_FX)
                (:Is%20Not%20Valid
                  (bind _returnvalue_2 (Game|SpawnActorfromClass "/Game/Blueprints/Weapons/BP_FX_Fire.BP_FX_Fire_C" (Math|Transform|MakeTransform "0, 0, 0") "Undefined" (Components|GetOwner) 0))
                  (Transformation|AttachComponentToComponent _returnvalue_2 (Variables|Default|GetSk_TP_Mesh) (Utilities|Name|MakeLiteralName "Muzzle") "SnapToTarget" "SnapToTarget" "SnapToTarget" true)
                  (bind _output_get_2 (Variables|Default|SetTP_FX _returnvalue_2))
                  (Default|SetOwnerNoSee _output_get_2))))))))
    (:then_1
      (if Hit
        (Effects|SpawnEmitteratLocation "/Game/MP_FPSBasic/Assets/MiscFX/Particles/PS_Rifle_Concrete_Impact.PS_Rifle_Concrete_Impact" _impactpoint (Math|Rotator|MakeRotfromZ _impactnormal))))))

(fn ReloadAddAmmo
  (Networking|SwitchHasAuthority
    (:Authority
      (bind _output_get (LocalVariables|SetAmmoNeedforReload (- (Variables|Default|GetMaxAmmoClipSize) (Variables|Default|GetCurrentAmmoInClip))))
      (if (<= (Variables|Default|GetCurrentMaxAmmo) _output_get)
        (Variables|Default|SetCurrentAmmoInClip (+ (Variables|Default|GetCurrentAmmoInClip) (Variables|Default|GetCurrentMaxAmmo)))
        (Variables|Default|SetCurrentMaxAmmo 0)
        (else
          (Variables|Default|SetCurrentMaxAmmo (- (Variables|Default|GetCurrentMaxAmmo) (LocalVariables|GetAmmoNeedforReload)))
          (Variables|Default|SetCurrentAmmoInClip (Variables|Default|GetMaxAmmoClipSize)))))))