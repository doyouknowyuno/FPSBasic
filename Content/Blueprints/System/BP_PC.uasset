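; BP_PC is a player controller that handles text chat and respawn requests.
; Enter focuses the chat widget's text box unless it already has keyboard focus.
; SendMessage prefixes the player's name and loops over every BP_PC, whose ReceiveMessagbe event updates its UMGChatting widget, which is not created here.
; Client_Respawn asks BP_GameMode to respawn this controller, which only works where the game mode exists, on the server.
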(event Custom|Client_Respawn
  (bind _returnvalue (Game|GetGameMode))
  (Utilities|IsValid _returnvalue
    (:Is%20Valid
      (bind _asbp_game_mode (Utilities|Casting|CastToBP_GameMode _returnvalue))
      (Default|RespawnPlayer _asbp_game_mode self))))

(event Custom|SendMessage
  (params (Message :type String))
  (bind _outactors (Actor|GetAllActorsOfClass "BP_PC_C"))
  (for _array_element _outactors
    (CallFunction|ReceiveMessagbe _array_element (Utilities|Text|ToText(String) (Utilities|String|Append (PlayerState|GetPlayerName (Variables|GetPlayerState)) " : " Message)))))

(event Custom|ReceiveMessagbe
  (params (Text :type Text))
  (Default|UpdateChat (Variables|Default|GetUMG_Chatting) Text))

(event EventBeginPlay)

(event EventTick
  (params (DeltaSeconds :type Float%20%28single-precision%29)))

(event Input|KeyboardEvents|Enter
  (params (Key :type Key%20Structure :default "None"))
  (bind _umg_chatting (Variables|Default|GetUMG_Chatting))
  (bind _editabletextbox_0 (Variables|/Game/Blueprints/Widgets/UMG_Chatting.UMG_Chatting_C|GetEditableTextBox_0 _umg_chatting))
  (:Pressed
    (Utilities|IsValid _umg_chatting
      (:Is%20Valid
        (if (not (Class|Widget|HasKeyboardFocus _editabletextbox_0))
          (Widget|SetFocus _editabletextbox_0))))))

(fn ConstructionScript)