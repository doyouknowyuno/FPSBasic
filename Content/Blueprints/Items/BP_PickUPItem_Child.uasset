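; BP_PickUPItem_Child is a pickup item that restores health to the overlapping actor.
; Its OnExplosivePickup event, despite the name, adds AmountToGive to CurrentHealth, clamped between zero and MaxHealth, then calls GetItem.
; An actor already at full health triggers neither the heal nor GetItem.
; The construction script only calls the parent, and the BeginPlay, overlap and Tick events are disabled placeholders.
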(event EventBeginPlay
  (|CallParentFunction) ; 지금 이 노드는 비활성 상태입니다. \n핀을 끌어서 다른 노드를 연결하면 활성화됩니다.
)

(event Collision|EventActorBeginOverlap
  (params (OtherActor :type Actor%20Object%20Reference))
  (|CallParentFunction OtherActor) ; 지금 이 노드는 비활성 상태입니다. \n핀을 끌어서 다른 노드를 연결하면 활성화됩니다.
)

(event EventTick
  (params (DeltaSeconds :type Float%20%28single-precision%29))
  (|CallParentFunction DeltaSeconds) ; 지금 이 노드는 비활성 상태입니다. \n핀을 끌어서 다른 노드를 연결하면 활성화됩니다.
)

(event EventOnExplosivePickup
  (params (OverlapActor :type BP%20Main%20Character%20Object%20Reference))
  (bind _maxhealth (Variables|/Game/Blueprints/Character/BP_MainCharacter.BP_MainCharacter_C|GetMaxHealth OverlapActor))
  (if (< (Variables|/Game/Blueprints/Character/BP_MainCharacter.BP_MainCharacter_C|GetCurrentHealth OverlapActor) _maxhealth)
    (Variables|/Game/Blueprints/Character/BP_MainCharacter.BP_MainCharacter_C|SetCurrentHealth OverlapActor (Math|Integer|Clamp(Integer) (+ (Variables|/Game/Blueprints/Character/BP_MainCharacter.BP_MainCharacter_C|GetCurrentHealth OverlapActor) (Variables|Default|GetAmountToGive)) 0 _maxhealth))
    (CallFunction|GetItem)))

(fn ConstructionScript
  (|CallParentFunction))