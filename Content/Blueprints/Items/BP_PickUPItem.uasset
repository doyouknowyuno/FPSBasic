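; BP_PickUPItem is an ammo pickup that refills the current weapon of an overlapping BP_MainCharacter, then respawns.
; On server-side overlap, OnExplosivePickup adds AmountToGive to CurrentMaxAmmo, clamped to MaxAmmo, only if it is below that limit.
; A successful pickup calls GetItem, which sets IsHidden for RespawnTime.
; The IsHidden RepNotify toggles actor visibility and Sphere collision, syncing availability to clients.
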(event Custom|OnExplosivePickup
  (params (OverlapActor :type BP%20Main%20Character%20Object%20Reference))
  (bind _currentweapon (Variables|/Game/Blueprints/Character/BP_MainCharacter.BP_MainCharacter_C|GetCurrentWeapon OverlapActor))
  (bind _maxammo (Variables|/Game/Blueprints/Weapons/BP_WeaponMaster.BP_WeaponMaster_C|GetMaxAmmo _currentweapon))
  (if (< (Variables|/Game/Blueprints/Weapons/BP_WeaponMaster.BP_WeaponMaster_C|GetCurrentMaxAmmo _currentweapon) _maxammo)
    (Variables|/Game/Blueprints/Weapons/BP_WeaponMaster.BP_WeaponMaster_C|SetCurrentMaxAmmo _currentweapon (Math|Integer|Clamp(Integer) (+ (Variables|/Game/Blueprints/Weapons/BP_WeaponMaster.BP_WeaponMaster_C|GetCurrentMaxAmmo _currentweapon) (Variables|Default|GetAmountToGive)) 0 _maxammo))
    (CallFunction|GetItem)))

(event Custom|GetItem
  (Variables|Default|SetIsHidden? true)
  (Utilities|FlowControl|Delay (Variables|Default|GetRespawnTime))
  (Variables|Default|SetIsHidden? false))

(event EventBeginPlay)

(event EventTick
  (params (DeltaSeconds :type Float%20%28single-precision%29)))

(event Collision|EventActorBeginOverlap
  (params (OtherActor :type Actor%20Object%20Reference))
  (Networking|SwitchHasAuthority
    (:Authority
      (bind _asbp_main_character (Utilities|Casting|CastToBP_MainCharacter OtherActor))
      (CallFunction|OnExplosivePickup _asbp_main_character))))

(fn ConstructionScript)

(fn OnRepIsHidden?
  (if (Variables|Default|GetIsHidden?)
    (Collision|SetCollisionEnabled (Variables|Default|GetSphere) "NoCollision")
    (Rendering|SetActorHiddenInGame true)
    (else
      (Collision|SetCollisionEnabled (Variables|Default|GetSphere) "QueryAndPhysics")
      (Rendering|SetActorHiddenInGame false))))